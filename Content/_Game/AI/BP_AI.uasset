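; BP_AI is an AI character that uses perception to notice the XR player pawn.
; On a perception update for that pawn, it sets the "hasSeenPlayer?" blackboard key to whether the pawn was successfully sensed.
; When sight is lost, it also stops movement immediately and resets its walk speed.
; It records its spawn location on BeginPlay.
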(event OnTargetPerceptionUpdated(AIPerception)
  (params (Actor :type Actor%20Object%20Reference) (Stimulus :type AI%20Stimulus%20Structure))
  (bind _self self)
  (bind _self_2 self)
  (bind _returnvalue (AI|GetAIController _self))
  (bind _charactermovement (Variables|Character|GetCharacterMovement _self_2))
  (bind _returnvalue_2 (AI|GetBlackboard _returnvalue))
  (Utilities|Casting|CastToBP_XRPawn Actor)
  (if (.bsuccessfullysensed Stimulus)
    (AI|Components|Blackboard|SetValueasBool _returnvalue_2 (Utilities|Name|MakeLiteralName "hasSeenPlayer?") true)
    (else
      (AI|Components|Blackboard|SetValueasBool _returnvalue_2 (Utilities|Name|MakeLiteralName "hasSeenPlayer?") false)
      (Components|Movement|StopMovementImmediately _charactermovement)
      (Variables|/Script/Engine.CharacterMovementComponent|SetMaxWalkSpeed _charactermovement 3e+02))))

(event EventBeginPlay
  (Variables|Default|SetSpawnLocation (Transformation|GetWorldLocation (Variables|Transformation|GetRootComponent))))

(fn ConstructionScript)