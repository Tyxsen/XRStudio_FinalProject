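; Player backpack actor, grabbable, with six child-actor inventory slots that opens a pair of windows in the level when all are filled.
; CheckInventoryFull, not called within this Blueprint, prints each stored item and sets IsInventoryFull.
; Tick fires the inventory-full event through a DoOnce that resets when no longer full.
; The handler bound at BeginPlay plays timelines that yaw the tag-found LeftWindow and RightWindow actors.
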(event Custom|InventoryIsFull_Event
  (bind _alpha (Timeline|LeftWindowTimeline Play)
    (:Update
      (Transformation|SetActorRelativeRotation (Variables|Default|GetLeftWindow) (Math|Rotator|MakeRotator 0.0 0.0 _alpha))
      (bind _alpha_2 (Timeline|RightWindowTimeline Play)
        (:Update
          (Transformation|SetActorRelativeRotation (Variables|Default|GetRightWindow) (Math|Rotator|MakeRotator 0.0 0.0 _alpha_2)))))))

(event EventBeginPlay
  (bind _asbp_inventory_component (Utilities|Casting|CastToBP_InventoryComponent (Variables|/Script/Engine.ChildActorComponent|GetChildActor (Variables|Default|GetBP_InventoryComponent1))))
  (Variables|Default|SetSlot1 _asbp_inventory_component)
  (bind _asbp_inventory_component_2 (Utilities|Casting|CastToBP_InventoryComponent (Variables|/Script/Engine.ChildActorComponent|GetChildActor (Variables|Default|GetBP_InventoryComponent2))))
  (Variables|Default|SetSlot2 _asbp_inventory_component_2)
  (bind _asbp_inventory_component_3 (Utilities|Casting|CastToBP_InventoryComponent (Variables|/Script/Engine.ChildActorComponent|GetChildActor (Variables|Default|GetBP_InventoryComponent3))))
  (Variables|Default|SetSlot3 _asbp_inventory_component_3)
  (bind _asbp_inventory_component_4 (Utilities|Casting|CastToBP_InventoryComponent (Variables|/Script/Engine.ChildActorComponent|GetChildActor (Variables|Default|GetBP_InventoryComponent4))))
  (Variables|Default|SetSlot4 _asbp_inventory_component_4)
  (bind _asbp_inventory_component_5 (Utilities|Casting|CastToBP_InventoryComponent (Variables|/Script/Engine.ChildActorComponent|GetChildActor (Variables|Default|GetBP_InventoryComponent5))))
  (Variables|Default|SetSlot5 _asbp_inventory_component_5)
  (bind _asbp_inventory_component_6 (Utilities|Casting|CastToBP_InventoryComponent (Variables|/Script/Engine.ChildActorComponent|GetChildActor (Variables|Default|GetBP_InventoryComponent6))))
  (Variables|Default|SetSlot6 _asbp_inventory_component_6)
  (bind _outactors (Actor|GetAllActorswithTag "LeftWindow"))
  (bind _array_element (Utilities|Array|ForEachLoopwithBreak _outactors)
    (:LoopBody
      (Variables|Default|SetLeftWindow _array_element)
      (bind _outactors_2 (Actor|GetAllActorswithTag "RightWIndow"))
      (bind _array_element_2 (Utilities|Array|ForEachLoopwithBreak _outactors_2)
        (:LoopBody
          (Variables|Default|SetRightWindow _array_element_2)
          (EventDispatchers|BindEventtoInventoryIsFull (delegate Custom|InventoryIsFull_Event)))))))

(event EventTick
  (params (DeltaSeconds :type Float%20%28single-precision%29))
  (if (Variables|Default|GetIsInventoryFull?)
    (Utilities|FlowControl|DoOnce false :!label _label
      (:Completed
        (CallFunction|InventoryIsFullEvent)))
    (else
      (goto _label Reset))))

(fn ConstructionScript)

(fn CheckInventoryFull
  (bind _slot4 (Variables|Default|GetSlot4))
  (bind _slot3 (Variables|Default|GetSlot3))
  (bind _slot1 (Variables|Default|GetSlot1))
  (bind _slot2 (Variables|Default|GetSlot2))
  (bind _slot5 (Variables|Default|GetSlot5))
  (bind _slot6 (Variables|Default|GetSlot6))
  (bind _storeditem (Variables|/Game/_Game/Blueprints/BP_InventoryComponent.BP_InventoryComponent_C|GetStoredItem _slot4))
  (bind _storeditem_2 (Variables|/Game/_Game/Blueprints/BP_InventoryComponent.BP_InventoryComponent_C|GetStoredItem _slot3))
  (bind _storeditem_3 (Variables|/Game/_Game/Blueprints/BP_InventoryComponent.BP_InventoryComponent_C|GetStoredItem _slot1))
  (bind _storeditem_4 (Variables|/Game/_Game/Blueprints/BP_InventoryComponent.BP_InventoryComponent_C|GetStoredItem _slot2))
  (bind _storeditem_5 (Variables|/Game/_Game/Blueprints/BP_InventoryComponent.BP_InventoryComponent_C|GetStoredItem _slot5))
  (bind _storeditem_6 (Variables|/Game/_Game/Blueprints/BP_InventoryComponent.BP_InventoryComponent_C|GetStoredItem _slot6))
  (Development|PrintString (Utilities|GetDisplayName _storeditem_3))
  (Development|PrintString (Utilities|GetDisplayName _storeditem_4))
  (Development|PrintString (Utilities|GetDisplayName _storeditem_2))
  (Development|PrintString (Utilities|GetDisplayName _storeditem))
  (Development|PrintString (Utilities|GetDisplayName _storeditem_5))
  (Development|PrintString (Utilities|GetDisplayName _storeditem_6))
  (if (Math|Boolean|ANDBoolean (Utilities|IsValid _storeditem_3) (Utilities|IsValid _storeditem_4) (Utilities|IsValid _storeditem_2) (Utilities|IsValid _storeditem) (Utilities|IsValid _storeditem_5) (Utilities|IsValid _storeditem_6))
    (Variables|Default|SetIsInventoryFull? true)
    (else
      (Variables|Default|SetIsInventoryFull? false))))

(fn IsGrabbable?
  (return true))