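; Small cube actor for the XR framework that marks itself as a grabbable object.
; Shortly after BeginPlay, it finds the static mesh component through its grabbable component's owner and switches it to the GrabbableObject collision profile.
; It prints the profile name before and after the change as debug output.
; Its IsGrabbable query always returns true.
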(event EventBeginPlay
  (bind _bp_grabbablecomponent (Variables|Default|GetBP_GrabbableComponent))
  (bind _returnvalue (Components|GetOwner _bp_grabbablecomponent))
  (bind _returnvalue_2 (Actor|GetComponentbyClass _returnvalue "/Script/Engine.StaticMeshComponent"))
  (bind _returnvalue_3 (Collision|GetCollisionProfileName _returnvalue_2))
  (Utilities|FlowControl|Delay 0.5)
  (Utilities|IsValid _returnvalue_2
    (:Is%20Valid
      (Development|PrintString (Utilities|String|ToString(Name) _returnvalue_3))
      (Collision|SetCollisionProfileName _returnvalue_2 "GrabbableObject" true :!class /Script/Engine.PrimitiveComponent)
      (Development|PrintString (Utilities|String|ToString(Name) _returnvalue_3)))))

(fn ConstructionScript)

(fn IsGrabbable?
  (return true))